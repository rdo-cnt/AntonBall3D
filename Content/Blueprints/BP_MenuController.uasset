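; BP_MenuController is an actor Blueprint that handles pause menu input and unpausing.
; MenuCancel forwards to the pause widget's CancelButtonPressed while the game is paused.
; UnpauseCheck either closes the menu, restoring game-only input with a sound, or cancels, depending on PauseState.
; The toggle chain that creates WBP_PauseMenu, focuses RESUME and pauses has no connected trigger, so it never runs here.
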(event Custom|UnpauseCheck
  (bind _returnvalue (Game|GetPlayerController 0))
  (bind _pausemenuref (Variables|Default|GetPauseMenuRef))
  ;[1 1 1] PauseButtonChoices
  (if (Utilities|Enum|Equal(Enum) (Variables|/Game/Blueprints/WBP_PauseMenu.WBP_PauseMenu_C|GetPauseState _pausemenuref) "NewEnumerator0")
    (Widget|RemovefromParent (Variables|Default|GetPauseMenuRef))
    (Game|SetGamePaused false)
    (Variables|/Script/Engine.PlayerController|SetbShowMouseCursor _returnvalue false)
    (Input|SetInputModeGameOnly _returnvalue)
    (Audio|PlaySound2D "/Game/Sounds/UI/snd_unpause.snd_unpause" 1.0 1.0 0.0 0 0)
    (else
      (Default|CancelButtonPressed _pausemenuref))))

(event EventBeginPlay)

(event Input|ActionEvents|InputActionMenuCancel
  (params (Key :type Key%20Structure :default "None"))
  (bind _pausemenuref (Variables|Default|GetPauseMenuRef))
  ;[1 1 1] B Button
  (:Pressed
    (Utilities|IsValid _pausemenuref
      (:Is%20Valid
        (if (Game|IsGamePaused)
          (Default|CancelButtonPressed _pausemenuref))))))

(event Input|ActionEvents|InputActionPause
  (params (Key :type Key%20Structure :default "None"))
  ;[1 1 1] Pause
)

(fn ConstructionScript)