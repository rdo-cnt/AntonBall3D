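; BP_Switch is a one-shot stage button that triggers ActivateObject on an assigned object when its Box is overlapped.
; Flags pick what can press it: an enemy mole in its Thrown state, a BP_DamageSource (dash attack), or any Character, with the mole flag overriding the dash one.
; If the target is valid, activation also recolors the point light and the button's dynamic material to DeactivatedColor.
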(event OnComponentBeginOverlap(Box)
  (params (OverlappedComponent :type Primitive%20Component%20Object%20Reference) (OtherActor :type Actor%20Object%20Reference) (OtherComp :type Primitive%20Component%20Object%20Reference) (OtherBodyIndex :type Integer) (bFromSweep :type Boolean) (SweepResult :type Hit%20Result%20Structure%20%28by%20ref%29))
  ;[1 1 1] Hit by Dash
  (if (Variables|Default|GetisMoleActivatedOnly%28MustBeOffForOtherActivationsToWork%29)
    (bind _asbp_enemy_mole (Utilities|Casting|CastToBP_EnemyMole OtherActor))
    ;[1 1 1] Button will only activate if mole is in "throwing" state
    (if true
      (switch Utilities|FlowControl|Switch|SwitchonEN_EnemyStates (Variables|/Game/Blueprints/CharacterActors/Enemies/BP_EnemyBase.BP_EnemyBase_C|GetEnumStates _asbp_enemy_mole)
        (:NewEnumerator11
          ;[1 1 1] Get dash attack
          (if (not (Variables|Default|Getactivated)) :!label _label
            (Variables|Default|Setactivated true)
            (CallFunction|ActivateObject)))))
    (else
      ;[1 1 1] Check if Button Should be Activated by Dash or Not
      (if (Variables|Default|GetIs%20Dash%20Activated%20Only)
        (Utilities|Casting|CastToBP_DamageSource OtherActor)
        (goto _label)
        (else
          ;[1 1 1] If no dash needed
          (Utilities|Casting|CastToCharacter OtherActor)
          (goto _label))))))

(event Custom|ActivateObject
  (bind _objecttoactivate (Variables|Default|GetobjectToActivate))
  (bind _pointlight (Variables|Default|GetPointLight))
  ;[1 1 1] Activate Object
  (Utilities|IsValid _objecttoactivate
    (:Is%20Valid
      (Default|ActivateObject _objecttoactivate)
      (Rendering|Components|Light|SetLightColor _pointlight (Math|Conversions|ToLinearColor(Color) (Variables|Default|GetDeactivatedColor)) true)
      (Rendering|Components|Light|SetIntensity _pointlight 5e+02)
      (Rendering|Material|SetVectorParameterValue (Variables|Default|GetChangeableMaterialInstance) "Param" (Math|Conversions|ToLinearColor(Color) (Variables|Default|GetDeactivatedColor)) :!class /Script/Engine.MaterialInstanceDynamic))))

(event EventBeginPlay
  (bind _returnvalue (Rendering|Material|CreateDynamicMaterialInstance (Variables|Default|GetMesh_Proto_Button) 1 0 "None" :!class /Script/Engine.PrimitiveComponent))
  (Variables|Default|SetChangeableMaterialInstance _returnvalue))

(fn ConstructionScript)