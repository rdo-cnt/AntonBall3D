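; Stage goal flag actor that triggers the player's victory when reached.
; Its Box overlap, ignored while Hidden, responds only to a BP_PlayerHurtBox and reaches the owning player through its ParentPlayer reference.
; It then plays that player's laugh sound, stops music through the GameInstance, hands the player's camera to the flag's Camera, and calls VictoryEvent.
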(event OnComponentBeginOverlap(Box)
  (params (OverlappedComponent :type Primitive%20Component%20Object%20Reference) (OtherActor :type Actor%20Object%20Reference) (OtherComp :type Primitive%20Component%20Object%20Reference) (OtherBodyIndex :type Integer) (bFromSweep :type Boolean) (SweepResult :type Hit%20Result%20Structure%20%28by%20ref%29))
  (if (not (Variables|Rendering|GetbHidden))
    (bind _asbp_player_hurt_box (Utilities|Casting|CastToBP_PlayerHurtBox OtherActor))
    (Audio|PlaySound2D (Variables|/Game/Blueprints/CharacterActors/BP_PlayerBase.BP_PlayerBase_C|GetlaughSoundCue (Variables|/Game/Blueprints/CharacterActors/BP_PlayerHurtBox.BP_PlayerHurtBox_C|GetParentPlayer _asbp_player_hurt_box)) 1.0 1.0 0.0 0 0)
    (Default|StopMusic (Variables|/Game/Blueprints/BP_AntonGameMode.BP_AntonGameMode_C|GetGameInstance (Variables|/Game/Blueprints/CharacterActors/BP_PlayerBase.BP_PlayerBase_C|GetGameMode (Variables|/Game/Blueprints/CharacterActors/BP_PlayerHurtBox.BP_PlayerHurtBox_C|GetParentPlayer _asbp_player_hurt_box))))
    (Default|SetNewCameraParent (Variables|/Game/Blueprints/CharacterActors/BP_PlayerHurtBox.BP_PlayerHurtBox_C|GetParentPlayer _asbp_player_hurt_box) (Variables|Default|GetCamera))
    (Default|VictoryEvent (Variables|/Game/Blueprints/CharacterActors/BP_PlayerHurtBox.BP_PlayerHurtBox_C|GetParentPlayer _asbp_player_hurt_box))))

(event EventBeginPlay)

(event Collision|EventActorBeginOverlap
  (params (OtherActor :type Actor%20Object%20Reference)))

(event EventTick
  (params (DeltaSeconds :type Float%20%28single-precision%29)))

(fn ConstructionScript)