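; Moving platform stage actor that travels out and back along a spline, optionally yawing with it.
; Once activated by a switch or at BeginPlay, it starts automatically or when a player steps on.
; A timeline scaled by movement time drives it, pausing at each end and repeating while auto-moving or occupied.
; The construction script picks tutorial or per-world materials and shows an optional box mesh, whose collision is set at BeginPlay.
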(event OnComponentBeginOverlap(Box)
  (params (OverlappedComponent :type Primitive%20Component%20Object%20Reference) (OtherActor :type Actor%20Object%20Reference) (OtherComp :type Primitive%20Component%20Object%20Reference) (OtherBodyIndex :type Integer) (bFromSweep :type Boolean) (SweepResult :type Hit%20Result%20Structure%20%28by%20ref%29))
  ;[1 1 1] Move when player enters the platform
  (Utilities|Casting|CastToBP_PlayerBase OtherActor)
  (Variables|Default|SethasPlayerOnTop true)
  (if (and (not (Variables|Default|GetisMoving)) (Variables|Default|GetActivated))
    (CallFunction|Move)))

(event OnComponentEndOverlap(Box)
  (params (OverlappedComponent :type Primitive%20Component%20Object%20Reference) (OtherActor :type Actor%20Object%20Reference) (OtherComp :type Primitive%20Component%20Object%20Reference) (OtherBodyIndex :type Integer))
  ;[1 1 1] Move when player enters the platform
  (Utilities|Casting|CastToBP_PlayerBase OtherActor)
  (Variables|Default|SethasPlayerOnTop false))

(event Custom|Move
  (bind _spline (Variables|Default|GetSpline))
  ;[1 1 1] Move around
  (bind _traveldistance (Timeline|MovePlatform Play)
    (:Update
      (Transformation|SetWorldLocation (Variables|Default|GetPlatformMesh) (Spline|GetLocationatDistanceAlongSpline _spline (* _traveldistance (Spline|GetSplineLength _spline)) "World") false false)
      (if (Variables|Default|GetRotateMeshWithSpline)
        (Transformation|SetRelativeRotation (Variables|Default|GetPlatformMesh) (Math|Rotator|MakeRotator 0.0 0.0 (.yaw (Spline|GetRotationatDistanceAlongSpline (Variables|Default|GetSpline) (* _traveldistance (Spline|GetSplineLength _spline)) "Local"))) false false)))
    (:Finished
      (Utilities|FlowControl|Delay (Variables|Default|GetstationaryTime))
      (if (Variables|Default|GetisMoving)
        (Variables|Default|SetisMoving false)
        (if (or (Variables|Default|GethasPlayerOnTop) (Variables|Default|GetautoMove))
          (CallFunction|Move))
        (else
          (Variables|Default|SetisMoving true)
          (CallFunction|MoveReverse))))))

(event Custom|MoveReverse
  (bind _spline (Variables|Default|GetSpline))
  ;[1 1 1] Move around
  (bind _traveldistance (Timeline|MovePlatform Reverse)
    (:Update
      (Transformation|SetWorldLocation (Variables|Default|GetPlatformMesh) (Spline|GetLocationatDistanceAlongSpline _spline (* _traveldistance (Spline|GetSplineLength _spline)) "World") false false)
      (if (Variables|Default|GetRotateMeshWithSpline)
        (Transformation|SetRelativeRotation (Variables|Default|GetPlatformMesh) (Math|Rotator|MakeRotator 0.0 0.0 (.yaw (Spline|GetRotationatDistanceAlongSpline (Variables|Default|GetSpline) (* _traveldistance (Spline|GetSplineLength _spline)) "Local"))) false false)))
    (:Finished
      (Utilities|FlowControl|Delay (Variables|Default|GetstationaryTime))
      (if (Variables|Default|GetisMoving)
        (Variables|Default|SetisMoving false)
        (if (or (Variables|Default|GethasPlayerOnTop) (Variables|Default|GetautoMove))
          (CallFunction|Move))
        (else
          (Variables|Default|SetisMoving true)
          (CallFunction|MoveReverse))))))

(event EventBeginPlay
  (bind _staticmesh (Variables|Default|GetStaticMesh))
  ;[1 1 1] Match rotation with first spline point
  (Components|Timeline|SetPlayRate (Variables|Default|GetMovePlatform) (/ 1.0 (Math|Float|Clamp(Float) (Variables|Default|GetmovementTime) 0.1 1e+04)))
  (Transformation|SetRelativeRotation (Variables|Default|GetPlatformMesh) (Math|Rotator|MakeRotator 0.0 0.0 (.yaw (Spline|GetRotationatDistanceAlongSpline (Variables|Default|GetSpline) 0.0 "Local"))) false false)
  (Utilities|FlowControl|Sequence
    (:then_0
      (if (Variables|Default|GetnoButtonNeeded)
        (CallFunction|ActivateObject)))
    (:then_1
      (if (Variables|Default|GethasBox)
        (Collision|SetCollisionEnabled _staticmesh "QueryAndPhysics")
        (else
          (Collision|SetCollisionEnabled _staticmesh "NoCollision"))))))

(event EventActivateObject
  ;[1 1 1] When activated by switch
  (Variables|Default|SetActivated true)
  (if (Variables|Default|GetautoMove)
    (CallFunction|Move)))

(fn ConstructionScript
  (bind _staticmesh (Variables|Default|GetStaticMesh))
  (bind _platformmesh (Variables|Default|GetPlatformMesh))
  (|CallParentFunction)
  (if (Variables|Default|GetisTutorialLevel)
    (Rendering|Material|SetMaterial _platformmesh 0 "/Game/Textures/MovingLevelObjectTextures/Platform/PlatformMesh/PlatformTutorialMesh_MAT.PlatformTutorialMesh_MAT")
    (if (Variables|Default|GethasBox) :!label _label
      (Rendering|SetVisibility _staticmesh true false)
      (else
        (Rendering|SetVisibility _staticmesh false false)))
    (if (Variables|Default|GetisTutorialLevel)
      (Rendering|Material|SetMaterial 0 0 "/Game/Textures/MovingLevelObjectTextures/Platform/Platform_01_MAT.Platform_01_MAT")
      (elif (Variables|Default|GetisWorld01)
        (Rendering|Material|SetMaterial _staticmesh 0 "/Game/Textures/MovingLevelObjectTextures/Platform/Platform_02_MAT.Platform_02_MAT")
        (elif (Variables|Default|GetisWorld02)
          (Rendering|Material|SetMaterial _staticmesh 0 "/Game/Textures/MovingLevelObjectTextures/Platform/Platform_03_MAT.Platform_03_MAT")
          (elif (Variables|Default|GetisWorld_03)
            (Rendering|Material|SetMaterial _staticmesh 0 "/Game/Textures/MovingLevelObjectTextures/Platform/Platform_04_MAT.Platform_04_MAT")
            (elif (Variables|Default|GetisWorld04)
              (Rendering|Material|SetMaterial _staticmesh 0 "/Game/Textures/MovingLevelObjectTextures/Platform/Platform_05_MAT.Platform_05_MAT")
              (elif (Variables|Default|GetisWorld05)
                (Rendering|Material|SetMaterial _staticmesh 0 "/Game/Textures/MovingLevelObjectTextures/Platform/Platform_06_MAT.Platform_06_MAT")))))))
    (elif (Variables|Default|GetisWorld01)
      (Rendering|Material|SetMaterial _platformmesh 0 "/Game/Textures/MovingLevelObjectTextures/Platform/PlatformMesh/PlatformWorld01Mesh_MAT.PlatformWorld01Mesh_MAT")
      (goto _label)
      (elif (Variables|Default|GetisWorld02)
        (Rendering|Material|SetMaterial _platformmesh 0 "/Game/Textures/MovingLevelObjectTextures/Platform/PlatformMesh/PlatformWorld02Mesh_MAT.PlatformWorld02Mesh_MAT")
        (goto _label)
        (elif (Variables|Default|GetisWorld_03)
          (Rendering|Material|SetMaterial _platformmesh 0 "/Game/Textures/MovingLevelObjectTextures/Platform/PlatformMesh/PlatformWorld03Mesh_MAT.PlatformWorld03Mesh_MAT")
          (goto _label)
          (elif (Variables|Default|GetisWorld04)
            (Rendering|Material|SetMaterial _platformmesh 0 "/Game/Textures/MovingLevelObjectTextures/Platform/PlatformMesh/PlatformWorld04Mesh_MAT.PlatformWorld04Mesh_MAT")
            (goto _label)
            (elif (Variables|Default|GetisWorld05)
              (Rendering|Material|SetMaterial _platformmesh 0 "/Game/Textures/MovingLevelObjectTextures/Platform/PlatformMesh/PlatformWorld05Mesh_MAT.PlatformWorld05Mesh_MAT")
              (goto _label))))))))