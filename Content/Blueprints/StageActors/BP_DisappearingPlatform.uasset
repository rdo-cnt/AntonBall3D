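; BP_DisappearingPlatform is a stage platform that blinks as a warning when a player steps on it and is meant to disappear.
; A box overlap with BP_PlayerBase starts Blink once, playing a timeline that drives a scalar parameter on the mesh's dynamic material instance.
; Blink calls Disappear only at zero blink count, but nothing here decrements it.
; Switch activation calls Reappear once; both Disappear and Reappear are empty.
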(event OnComponentBeginOverlap(Box)
  (params (OverlappedComponent :type Primitive%20Component%20Object%20Reference) (OtherActor :type Actor%20Object%20Reference) (OtherComp :type Primitive%20Component%20Object%20Reference) (OtherBodyIndex :type Integer) (bFromSweep :type Boolean) (SweepResult :type Hit%20Result%20Structure%20%28by%20ref%29))
  ;[1 1 1] Threaten player when stepped on
  (Utilities|Casting|CastToBP_PlayerBase OtherActor)
  (if (not (Variables|Default|GetSteppedOnPlatform))
    (Variables|Default|SetSteppedOnPlatform true)
    (Variables|Default|SetblinkCount (Variables|Default|GetblinkAmount))
    (CallFunction|Blink)))

(event Custom|Disappear
  ;[1 1 1] Appearing and disappearing
)

(event Custom|Reappear
  ;[1 1 1] Appearing and disappearing
)

(event Custom|Blink
  ;[1 1 1] BlinkingProcess
  (if (> (Variables|Default|GetblinkCount) 0)
    (bind _newtrack_0 (Timeline|Timeline_0 Play)
      (:Update
        (Rendering|Material|SetScalarParameterValue (Variables|Default|GetChangeableMaterialInstance) (Variables|Default|GetParameter%20Name) _newtrack_0 :!class /Script/Engine.MaterialInstanceDynamic)))
    (else
      (CallFunction|Disappear))))

(event EventBeginPlay
  ;[1 1 1] Start
  (Variables|Default|SetblinkCount (Variables|Default|GetblinkAmount))
  (bind _returnvalue (Rendering|Material|CreateDynamicMaterialInstance (Variables|Default|GetPlatformMesh) 1 0 "None" :!class /Script/Engine.PrimitiveComponent))
  (Variables|Default|SetChangeableMaterialInstance _returnvalue))

(event EventActivateObject
  ;[1 1 1] When activated by switch
  (if (not (Variables|Default|GetActivated))
    (Variables|Default|SetActivated true)
    (CallFunction|Reappear)))

(fn ConstructionScript
  (|CallParentFunction))