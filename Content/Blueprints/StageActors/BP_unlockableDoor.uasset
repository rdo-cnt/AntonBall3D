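; Unlockable door stage actor that slides its door mesh upward when activated.
; ActivateObject sets the Activated flag and calls Move, which also runs on BeginPlay if the flag is already set.
; Move captures the mesh's world location, then plays the Opendoor timeline to lerp it to a fixed height above that start, without sweeping.
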(event Custom|Move
  (bind _output_get (Variables|Default|SetStart%20Location (Transformation|GetWorldLocation (Variables|Default|Getdoormesh))))
  (Variables|Default|SetEnd%20Location (+ _output_get "0,0.000000,400.000000"))
  (bind _opendoor (Timeline|opendoor Play)
    (:Update
      (Transformation|SetWorldLocation (Variables|Default|Getdoormesh) (Math|Vector|Lerp(Vector) (Variables|Default|GetStart%20Location) (Variables|Default|GetEnd%20Location) _opendoor) false false))))

(event EventBeginPlay
  (if (Variables|Default|GetActivated)
    (CallFunction|Move)))

(event Collision|EventActorBeginOverlap
  (params (OtherActor :type Actor%20Object%20Reference)))

(event EventTick
  (params (DeltaSeconds :type Float%20%28single-precision%29)))

(event EventActivateObject
  (Variables|Default|SetActivated true)
  (CallFunction|Move))

(fn ConstructionScript
  (|CallParentFunction))