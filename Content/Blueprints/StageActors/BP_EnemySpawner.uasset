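; Pipe stage actor that spawns an AI enemy and spits it out when the player first enters its detection area.
; The first overlap creates the enemy with BT_Mole, passes it the patrol points, then enables and launches it along the spawn point's forward vector.
; A reset event calls the mole's spawner reset.
; Dynamic materials tint both pipe meshes at BeginPlay and on editor tick for live preview.
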(event OnComponentBeginOverlap(PlayerDetector)
  (params (OverlappedComponent :type Primitive%20Component%20Object%20Reference) (OtherActor :type Actor%20Object%20Reference) (OtherComp :type Primitive%20Component%20Object%20Reference) (OtherBodyIndex :type Integer) (bFromSweep :type Boolean) (SweepResult :type Hit%20Result%20Structure%20%28by%20ref%29))
  ;[0.1602 0.3842 1] If Anton is close, spawn first enemy
  (Utilities|Casting|CastToBP_PlayerBase OtherActor)
  (if (not (Variables|Default|GethasSpawnedFirstEnemy))
    (CallFunction|CreateEnemy)
    (CallFunction|SpawnEnemy)
    (Variables|Default|SethasSpawnedFirstEnemy true)))

(event Custom|Create%20Enemy
  (bind _spawnpoint (Variables|Default|GetSpawnPoint))
  (bind _returnvalue (Transformation|GetWorldTransform _spawnpoint))
  ;[0.4094 0.2216 1] Create Enemy for the enemy container
  (bind _returnvalue_2 (AI|SpawnAIFromClass (Variables|Default|GetEnemySpawnObject) "/Game/Blueprints/CharacterActors/Enemies/BT_Mole.BT_Mole" (.location _returnvalue) (.rotation _returnvalue) false 0))
  (bind _asbp_enemy_base (Utilities|Casting|CastToBP_EnemyBase _returnvalue_2))
  (bind _output_get (Variables|Default|SetEnemyReference _asbp_enemy_base))
  (Variables|/Game/Blueprints/CharacterActors/Enemies/BP_EnemyBase.BP_EnemyBase_C|SetPatrolPoints _output_get (Variables|Default|GetPatrolPoints)))

(event Custom|SpawnEnemy
  (bind _spawnpoint (Variables|Default|GetSpawnPoint))
  (bind _enemyreference (Variables|Default|GetEnemyReference))
  (bind _returnvalue (Transformation|GetWorldRotation _spawnpoint))
  ;[1 0.1094 0.1094] Spit Enemy
  (Transformation|SetWorldLocation (Variables|/Script/Engine.Character|GetCapsuleComponent _enemyreference) (Transformation|GetWorldLocation _spawnpoint) false false)
  (Default|EnableEnemy _enemyreference)
  (Character|LaunchCharacter _enemyreference (* (Math|Vector|GetForwardVector _returnvalue) (Variables|Default|GetLaunchForce)) true true)
  (Transformation|SetActorRotation _enemyreference (Math|Rotator|MakeRotator 0.0 0.0 (.Yaw (Math|Rotator|BreakRotator _returnvalue)))))

(event Custom|ChangeColor
  ;[1 1 1] ChangeColor
  (bind _returnvalue (Rendering|Material|CreateDynamicMaterialInstance (Variables|Default|GetStaticMesh) 0 0 "None" :!class /Script/Engine.PrimitiveComponent))
  (Rendering|Material|SetVectorParameterValue _returnvalue "Param" (Math|Conversions|ToLinearColor(Color) (Variables|Default|GetPipeColor)) :!class /Script/Engine.MaterialInstanceDynamic)
  (bind _returnvalue_2 (Rendering|Material|CreateDynamicMaterialInstance (Variables|Default|GetStaticMesh1) 0 0 "None" :!class /Script/Engine.PrimitiveComponent))
  (Rendering|Material|SetVectorParameterValue _returnvalue_2 "Param" (Math|Conversions|ToLinearColor(Color) (Variables|Default|GetPipeColor)) :!class /Script/Engine.MaterialInstanceDynamic))

(event Custom|EnemyResetDie
  (bind _asbp_enemy_mole (Utilities|Casting|CastToBP_EnemyMole (Variables|Default|GetEnemyReference)))
  (Default|Moleresetspawner _asbp_enemy_mole))

(event EventBeginPlay
  (CallFunction|ChangeColor))

(event Collision|EventActorBeginOverlap
  (params (OtherActor :type Actor%20Object%20Reference)))

(event EventEditorTick
  ;[1 1 1] EDITOR: color pipes
  (CallFunction|ChangeColor))

(fn ConstructionScript
  (AddComponent|AddChildActorComponent false))