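; Menu pawn that sets up the main menu UI and mouse input when play begins.
; BeginPlay creates WBP_MainMenu2, sets its pause state, calls ChangeFocusable, shows the cursor and switches to Game and UI input focused on the widget, with the mouse locked in fullscreen.
; It also gathers CameraActors without using them; the view-target blend and Antonball welcome track are disconnected and never run.
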(event EventBeginPlay
  (bind _returnvalue (Game|GetPlayerController 0))
  (bind _returnvalue_2 (UserInterface|CreateWidget "/Game/Blueprints/WBP_MainMenu2.WBP_MainMenu2_C"))
  (bind _output_get (Variables|Default|SetMainMenu_0 _returnvalue_2))
  (Variables|/Game/Blueprints/WBP_MainMenu2.WBP_MainMenu2_C|SetPauseState _output_get "NewEnumerator4")
  (Default|ChangeFocusable _output_get)
  (Variables|/Script/Engine.PlayerController|SetbShowMouseCursor _returnvalue true)
  (bind _outactors (Actor|GetAllActorsOfClass "/Script/Engine.CameraActor"))
  (Input|SetInputModeGameandUI _returnvalue _returnvalue_2 "LockInFullscreen" true))

(event Collision|EventActorBeginOverlap
  (params (OtherActor :type Actor%20Object%20Reference)))

(event EventTick
  (params (DeltaSeconds :type Float%20%28single-precision%29)))

(fn ConstructionScript)