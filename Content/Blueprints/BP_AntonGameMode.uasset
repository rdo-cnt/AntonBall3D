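; BP_AntonGameMode is the game mode for AntonGame, holding references to the game instance, score manager and player.
; On BeginPlay it casts and caches BP_AntonGame_GameInstance, then spawns a BP_AntonGame_ScoreManager at the world origin and stores it.
; ReceiveCharacter stores the player reference passed to it, and GoToNextLevel forwards level changes to the game instance.
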(event Custom|GoToNextLevel
  ;[1 1 1] Move to the next level
  (Default|GotoNextLevel (Variables|Default|GetGameInstance)))

(event Custom|ReceiveCharacter
  (params (Player :type BP%20Player%20Base%20Object%20Reference))
  ;[1 1 1] Get Character Function
  (Variables|Default|SetPlayer Player))

(event Custom|GenerateManagers
  ;[1 1 1] Generate Temporary Managers
  (bind _returnvalue (Game|SpawnActorfromClass "/Game/Blueprints/BP_AntonGame_ScoreManager.BP_AntonGame_ScoreManager_C" (Math|Transform|MakeTransform "0, 0, 0") "Undefined" 0 0))
  (Variables|Default|SetScoreManager _returnvalue))

(event EventBeginPlay
  ;[1 1 1] Startup
  (bind _asbp_anton_game_game_instance (Utilities|Casting|CastToBP_AntonGame_GameInstance (Game|GetGameInstance)))
  (Variables|Default|SetGameInstance _asbp_anton_game_game_instance)
  (CallFunction|GenerateManagers))

(event EventTick
  (params (DeltaSeconds :type Float%20%28single-precision%29)))

(fn ConstructionScript)