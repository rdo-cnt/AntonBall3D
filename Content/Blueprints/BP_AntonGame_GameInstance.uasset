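; Game instance for AntonGame that owns the save game, handling persistent graphics settings, per-level high scores and level progression.
; Init loads or creates the "Slot" save, applies quality settings through console commands, then pads the per-level score and collectible arrays to match LevelList.
; Save events write each setting, and CompareSaveScore stores scores beating the current level's record.
; GoToNextLevel opens maps by LevelList key order, while StreamLevel loads sublevels.
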(event Custom|GoToNextLevel
  (bind _levellist (Variables|Default|GetLevelList))
  ;[1 1 1] Move to the next level
  (bind _values (Utilities|Map|Values _levellist))
  (bind _result (Math|Integer|IncrementInt (Variables|Default|GetCurrentLevel))
    (:%20%20
      (if (> _result (Utilities|Array|Length _values))
        (Variables|Default|SetCurrentLevel 0))
      (bind _keys (Utilities|Map|Keys _levellist))
      (Game|OpenLevel(byObjectReference) (Utilities|Array|Get(acopy) _keys (Variables|Default|GetCurrentLevel))))))

(event Custom|StreamLevel
  (params (LevelName :type Name))
  ;[1 1 1] StreamLevel
  ;;[1 1 1] LoadLevelFirst
  (Game|LoadStreamLevel(byName) LevelName true true)
  (Utilities|FlowControl|Delay 0.2))

(event Custom|SaveTextureQuality
  (params (index :type Integer))
  (bind _savegame (Variables|Default|GetSaveGame))
  ;[1 1 1] SaveTextureQuality
  (Variables|/Game/Blueprints/SaveGameStuff.SaveGameStuff_C|SetTextureIndex _savegame index)
  (SaveGame|SaveGametoSlot _savegame "slot"))

(event Custom|SaveAntiAlias
  (params (index :type Integer))
  (bind _savegame (Variables|Default|GetSaveGame))
  ;[1 1 1] SaveAntiAlias
  (Variables|/Game/Blueprints/SaveGameStuff.SaveGameStuff_C|SetAntiAliasIndex _savegame index)
  (SaveGame|SaveGametoSlot _savegame "slot"))

(event Custom|CheckLevelDictionaries
  (bind _savegame (Variables|Default|GetSaveGame))
  (bind _savegame_2 (Variables|Default|GetSaveGame))
  (bind _levelhiscore (Variables|/Game/Blueprints/SaveGameStuff.SaveGameStuff_C|GetLevelHiScore _savegame))
  (bind _returnvalue (Utilities|Array|Length _levelhiscore))
  ;[1 1 1] Create Save file level dictionary
  (bind _keys (Utilities|Map|Keys (Variables|Default|GetLevelList)))
  ;;[1 1 1] If our map list is bigger than our saved list, match the length
  (if (> (Utilities|Array|Length _keys) _returnvalue) :!label _label
    (Variables|Default|SetLevelListCounterForSave _returnvalue)
    (Utilities|Array|Add (Variables|/Game/Blueprints/SaveGameStuff.SaveGameStuff_C|GetLevelHiScore _savegame_2) 0)
    (Utilities|Array|Add (Variables|/Game/Blueprints/SaveGameStuff.SaveGameStuff_C|GetLevelCollectibleList _savegame_2) (Variables|Default|GetBaseLevelCollectibleList))
    (goto _label)
    (else
      (SaveGame|SaveGametoSlot (Variables|Default|GetSaveGame) "Slot"))))

(event Custom|SaveScreenResolution
  (params (String :type String))
  ;[1 1 1] SaveScreenResolution
  (Variables|/Game/Blueprints/SaveGameStuff.SaveGameStuff_C|SetResolution (Variables|Default|GetSaveGame) String)
  (SaveGame|SaveGametoSlot (Variables|Default|GetSaveGame) "slot"))

(event Custom|CompareSaveScore
  (bind _savegame (Variables|Default|GetSaveGame))
  (bind _levelhiscore (Variables|/Game/Blueprints/SaveGameStuff.SaveGameStuff_C|GetLevelHiScore _savegame))
  ;[1 1 1] Compare Scores
  (bind _asbp_anton_game_mode (Utilities|Casting|CastToBP_AntonGameMode (Game|GetGameMode)))
  (if (> (Variables|/Game/Blueprints/BP_AntonGame_ScoreManager.BP_AntonGame_ScoreManager_C|GetScore (Variables|/Game/Blueprints/BP_AntonGameMode.BP_AntonGameMode_C|GetScoreManager _asbp_anton_game_mode)) (Utilities|Array|Get(acopy) _levelhiscore (Variables|Default|GetCurrentLevel)))
    (Utilities|Array|SetArrayElem _levelhiscore (Variables|Default|GetCurrentLevel) (Variables|/Game/Blueprints/BP_AntonGame_ScoreManager.BP_AntonGame_ScoreManager_C|GetScore (Variables|/Game/Blueprints/BP_AntonGameMode.BP_AntonGameMode_C|GetScoreManager _asbp_anton_game_mode)))
    (SaveGame|SaveGametoSlot (Variables|Default|GetSaveGame) "slot")))

(event Custom|CheckScreenResolution
  ;[1 1 1] CheckForScreenResolution
  (if (Utilities|Enum|Equal(Enum) (Variables|/Game/Blueprints/SaveGameStuff.SaveGameStuff_C|GetResolution (Variables|Default|GetSaveGame)) "")
    (bind _returnvalue (Settings|GetGameUserSettings))
    (CallFunction|SaveScreenResolution (Utilities|String|Append (Utilities|String|ToString(Integer) (.X (Utilities|Struct|BreakIntPoint (Class|GameUserSettings|GetScreenResolution _returnvalue)))) " x " (Utilities|String|ToString(Integer) (.Y (Utilities|Struct|BreakIntPoint (Class|GameUserSettings|GetScreenResolution _returnvalue))))))
    (Development|ExecuteConsoleCommand (Utilities|String|Append "r.setres " (Utilities|String|Replace (Utilities|String|Append (Utilities|String|ToString(Integer) (.X (Utilities|Struct|BreakIntPoint (Class|GameUserSettings|GetScreenResolution _returnvalue)))) " x " (Utilities|String|ToString(Integer) (.Y (Utilities|Struct|BreakIntPoint (Class|GameUserSettings|GetScreenResolution _returnvalue))))) " ")) 0)))

(event Custom|Settings%20Check
  ;[1 1 1] Settings Check
  (CallFunction|CheckScreenResolution)
  (CallFunction|SettingsQualities))

(event Custom|SettingsQualities
  ;[1 1 1] Check for settings qualities
  (Development|ExecuteConsoleCommand (Utilities|String|Append "sg.TextureQuality " (Utilities|String|ToString(Integer) (Variables|/Game/Blueprints/SaveGameStuff.SaveGameStuff_C|GetTextureIndex (Variables|Default|GetSaveGame)))) 0)
  (Development|ExecuteConsoleCommand (Utilities|String|Append "sg.ShadowQuality " (Utilities|String|ToString(Integer) (Variables|/Game/Blueprints/SaveGameStuff.SaveGameStuff_C|GetShadowIndex (Variables|Default|GetSaveGame)))) 0)
  (Development|ExecuteConsoleCommand (Utilities|String|Append "r.PostProcessAAQuality " (Utilities|String|ToString(Integer) (Variables|/Game/Blueprints/SaveGameStuff.SaveGameStuff_C|GetAntiAliasIndex (Variables|Default|GetSaveGame)))) 0))

(event Custom|SaveShadowQuality
  (params (index :type Integer))
  (bind _savegame (Variables|Default|GetSaveGame))
  ;[1 1 1] SaveShadowQuality
  (Variables|/Game/Blueprints/SaveGameStuff.SaveGameStuff_C|SetShadowIndex _savegame index)
  (SaveGame|SaveGametoSlot _savegame "slot"))

(event EventInit
  ;[0 0.236 1] Create Modular Instances
  ;;[1 0.4576 0] Save Stuff
  (bind _returnvalue (SaveGame|DoesSaveGameExist "Slot"))
  (if _returnvalue
    (bind _returnvalue_2 (SaveGame|LoadGamefromSlot "Slot"))
    (bind _assave_game_stuff (Utilities|Casting|CastToSaveGameStuff _returnvalue_2))
    (Variables|Default|SetSaveGame _assave_game_stuff)
    (else
      (bind _returnvalue_3 (SaveGame|CreateSaveGameObject "/Game/Blueprints/SaveGameStuff.SaveGameStuff_C"))
      (Variables|Default|SetSaveGame _returnvalue_3)))
  (CallFunction|SettingsCheck)
  (CallFunction|CheckLevelDictionaries)
  (for _array_element (Variables|/Game/Blueprints/SaveGameStuff.SaveGameStuff_C|GetLevelHiScore (Variables|Default|GetSaveGame))
    (Development|PrintString (Utilities|String|ToString(Integer) _array_element))))

(fn ReturnStageScore
  (return (Utilities|Array|Get(acopy) (Variables|/Game/Blueprints/SaveGameStuff.SaveGameStuff_C|GetLevelHiScore (Variables|Default|GetSaveGame)) (Variables|Default|GetCurrentLevel))))