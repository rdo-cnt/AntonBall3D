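; Rotating block actor that repeatedly turns its static mesh in quarter-turn yaw steps, clockwise or counter-clockwise per IsClockwise.
; Rotation starts on BeginPlay if Activated is set, or when ActivateObject is called.
; Each step lerps the mesh's relative rotation through a timeline, then waits RotationDelay and loops from the new orientation indefinitely.
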(event Custom|RotationEvent
  (bind _staticmesh (Variables|Default|GetStaticMesh))
  (bind _relativerotation (Variables|/Script/Engine.SceneComponent|GetRelativeRotation _staticmesh))
  (bind (_roll _pitch) (Math|Rotator|BreakRotator _relativerotation))
  ;[1 1 1] Rotating Block
  ;;[1 1 1] Check if block spins clockwise or counter clockwise
  (if (Variables|Default|GetIs%20Clockwise?)
    ;;[1 1 1] Set Block Rotation +/-90 degrees every loop
    (Variables|Default|SetDegree 9e+01)
    (else
      (Variables|Default|SetDegree -9e+01)))
  (bind _output_get (Variables|Default|SetStart _relativerotation :!label _label))
  (Variables|Default|SetEnd (Math|Rotator|CombineRotators _output_get (Math|Rotator|MakeRotator _roll _pitch (Variables|Default|GetDegree))))
  ;;[1 1 1] While timeline plays, lerp between (start) set and (end) set variable values and delay before looping rotation again
  (bind _0_1 (Timeline|rotatoe PlayFromStart)
    (:Update
      (Transformation|SetRelativeRotation (Variables|Default|GetStaticMesh) (Math|Rotator|Lerp(Rotator) (Variables|Default|GetStart) (Variables|Default|GetEnd) _0_1 true) false false))
    (:Finished
      (Utilities|FlowControl|Delay (Variables|Default|GetRotation%20Delay))
      (goto _label))))

(event EventBeginPlay
  (if (Variables|Default|GetActivated)
    (CallFunction|RotationEvent)))

(event Collision|EventActorBeginOverlap
  (params (OtherActor :type Actor%20Object%20Reference))
  ;[1 1 1] Rotating Block
)

(event EventTick
  (params (DeltaSeconds :type Float%20%28single-precision%29))
  ;[1 1 1] Rotating Block
)

(event EventActivateObject
  (Variables|Default|SetActivated true)
  (CallFunction|RotationEvent))

(fn ConstructionScript)