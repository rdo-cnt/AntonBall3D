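; ExtraCoin is a spinning pickup actor that awards extra coins when it overlaps a BP_PlayerHurtBox.
; BeginPlay drives the spin with a looping Delay of one frame's delta time instead of using Tick.
; On pickup it plays one of three random laugh sounds, prints a separately rolled debug number, adds its coin amount through the GameMode's ScoreManager, then destroys itself.
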(event EventBeginPlay
  (bind _returnvalue (Utilities|Time|GetWorldDeltaSeconds))
  ;[1 1 1] On Start
  (Transformation|AddActorLocalRotation (Math|Rotator|MakeRotator 0.0 0.0 (* (Variables|Default|GetRotationPerSecond) _returnvalue)) false false :!label _label)
  (Utilities|FlowControl|Delay _returnvalue)
  (goto _label))

(event Collision|EventActorBeginOverlap
  (params (OtherActor :type Actor%20Object%20Reference))
  (bind _returnvalue (Math|Random|RandomInteger 3))
  (bind _asbp_player_hurt_box (Utilities|Casting|CastToBP_PlayerHurtBox OtherActor))
  ;[1 1 1] Add Coin to score
  (Math|Integer|CompareInt _returnvalue 1
    (:>
      (Audio|PlaySound2D "/Game/Sounds/Player/Anton/snd_anton_prelaugh.snd_anton_prelaugh" 1.0 1.0 0.0 0 0))
    (:==
      (Audio|PlaySound2D "/Game/Sounds/Player/Anton/snd_anton_laugh.snd_anton_laugh" 1.0 1.0 0.0 0 0))
    (:<
      (Audio|PlaySound2D "/Game/Sounds/Player/Anton/snd_anton_laugh2.snd_anton_laugh2" 1.0 1.0 0.0 0 0)))
  (Development|PrintString (Utilities|String|ToString(Integer) _returnvalue))
  (Default|AddExtraCoin (Variables|/Game/Blueprints/BP_AntonGameMode.BP_AntonGameMode_C|GetScoreManager (Variables|/Game/Blueprints/CharacterActors/BP_PlayerBase.BP_PlayerBase_C|GetGameMode (Variables|/Game/Blueprints/CharacterActors/BP_PlayerHurtBox.BP_PlayerHurtBox_C|GetParentPlayer _asbp_player_hurt_box))) (Variables|Default|GetExtraCointAmount))
  (Actor|DestroyActor))

(fn ConstructionScript)