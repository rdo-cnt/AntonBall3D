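; BP_AntonAfterImage is a short-lived afterimage actor, presumably for the Anton character, shown as a randomly tinted static mesh.
; On BeginPlay it creates a dynamic material instance on the mesh and picks a color at random from RandomColor.
; A timeline writes that color to a vector parameter while animating its alpha, then destroys the actor when finished.
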(event Custom|TimelineMat
  (bind _color (Variables|Default|GetColor))
  (bind _newtrack_0 (Timeline|Timeline_0 Play)
    (:Update
      (Rendering|Material|SetVectorParameterValue (Variables|Default|GetMaterial%20Instance) "Param" (Utilities|Struct|MakeLinearColor (Math|Conversions|ToFloat(Byte) (.r _color)) (Math|Conversions|ToFloat(Byte) (.g _color)) (Math|Conversions|ToFloat(Byte) (.b _color)) _newtrack_0) :!class /Script/Engine.MaterialInstanceDynamic))
    (:Finished
      (Actor|DestroyActor))))

(event EventBeginPlay
  (bind _returnvalue (Rendering|Material|CreateDynamicMaterialInstance (Variables|Default|GetStaticMesh) 0 0 "None" :!class /Script/Engine.PrimitiveComponent))
  (Variables|Default|SetMaterial%20Instance _returnvalue)
  (Variables|Default|SetColor (.OutItem (Utilities|Array|Random (Variables|Default|GetRandomColor))))
  (CallFunction|TimelineMat))

(event Collision|EventActorBeginOverlap
  (params (OtherActor :type Actor%20Object%20Reference)))

(event EventTick
  (params (DeltaSeconds :type Float%20%28single-precision%29)))

(fn ConstructionScript)