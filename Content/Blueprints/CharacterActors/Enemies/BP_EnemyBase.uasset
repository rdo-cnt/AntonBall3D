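; Base enemy character providing shared state, stun, hitbox and respawn plumbing, with empty death, stun-recovery and per-state tick logic.
; GetHurt stuns roaming, spotting or chasing enemies, which become grabbable once invincibility expires; both countdowns use frame-length Delay loops.
; Respawning waits, then restores the starting transform and re-enables the enemy if testing or its spawner is valid.
; Helpers toggle collision, gravity and a child-actor damage hitbox.
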(event Custom|ActivateHitbox
  ;[1 1 1] Hitboxes
  (bind _asbp_enemy_damage_source (Utilities|Casting|CastToBP_EnemyDamageSource (Variables|/Script/Engine.ChildActorComponent|GetChildActor (Variables|Default|GetChildActor))))
  (Default|ActivateCollision _asbp_enemy_damage_source))

(event Custom|DeactivateHitbox
  ;[1 1 1] Hitboxes
  (bind _asbp_enemy_damage_source (Utilities|Casting|CastToBP_EnemyDamageSource (Variables|/Script/Engine.ChildActorComponent|GetChildActor (Variables|Default|GetChildActor))))
  (Development|PrintString "Hello")
  (Default|DeactivateCollision _asbp_enemy_damage_source))

(event Custom|Respawning
  ;[1 1 1] Respawning
  (Utilities|FlowControl|Delay (Variables|Default|GetRespawnTime))
  (CallFunction|ResetEnemy))

(event Custom|DeathEvent
  ;[1 1 1] Death CustomEvent
)

(event Custom|Spawn%20Tick
  ;[1 1 1] Tick Events
  (if (AI|Components|NavMovement|IsMovingonGround (Variables|Character|GetCharacterMovement))
    (Variables|Default|SetEnumStates "NewEnumerator5")))

(event Custom|Enable%20Enemy
  (Rendering|SetActorHiddenInGame false)
  (Collision|SetCollisionEnabled (Variables|Collision|GetCapsuleComponent) "QueryAndPhysics")
  (Actor|Tick|SetActorTickEnabled true)
  (Variables|Default|SetEnumStates "NewEnumerator0"))

(event Custom|InvincibilityTimer
  (bind _returnvalue (Utilities|Time|GetWorldDeltaSeconds))
  ;[1 1 1] CountInvincibilityTimer
  (if (> (Variables|Default|GetinvincibilityCountdown) 0.0) :!label _label
    (Variables|Default|SetinvincibilityCountdown (- (Variables|Default|GetinvincibilityCountdown) _returnvalue))
    (Utilities|FlowControl|Delay _returnvalue)
    (goto _label)))

(event Custom|Disable%20Enemy
  (Rendering|SetActorHiddenInGame true)
  (Collision|SetCollisionEnabled (Variables|Collision|GetCapsuleComponent) "NoCollision")
  (Actor|Tick|SetActorTickEnabled false))

(event Custom|CountStunTimer
  (bind _returnvalue (Utilities|Time|GetWorldDeltaSeconds))
  ;[1 1 1] Count Stun Time
  (if (> (Variables|Default|GetstunTimeCountdown) 0.0) :!label _label
    (Variables|Default|SetstunTimeCountdown (- (Variables|Default|GetstunTimeCountdown) _returnvalue))
    (Utilities|FlowControl|Delay _returnvalue)
    (goto _label)
    (else
      (CallFunction|SpringBacktoAction))))

(event Custom|EnableGravity
  ;[1 1 1] Enable/Disable Gravity
  (Variables|/Script/Engine.CharacterMovementComponent|SetGravityScale (Variables|Character|GetCharacterMovement) (Variables|Default|GetGravityBase)))

(event Custom|DisableCollision
  ;[1 1 1] Disable Collisions
  (Collision|SetCollisionEnabled (Variables|Collision|GetCapsuleComponent) "NoCollision")
  (CallFunction|DeactivateHitbox))

(event Custom|EnableCollision
  ;[1 1 1] Disable Collisions
  (Collision|SetCollisionEnabled (Variables|Collision|GetCapsuleComponent) "QueryAndPhysics"))

(event Custom|SpringBackToAction
  ;[1 1 1] Spring Back to action
)

(event Custom|LandingTick
  ;[1 1 1] Tick Events
  (bind _output_get (Variables|Default|SetWaitAfterLandingCooldown (- (Variables|Default|GetWaitAfterLandingTime) (Utilities|Time|GetWorldDeltaSeconds))))
  (if (<= _output_get 0.0)
    (Variables|Default|SetEnumStates "NewEnumerator0")))

(event Custom|DisableGravity
  ;[1 1 1] Enable/Disable Gravity
  (Variables|/Script/Engine.CharacterMovementComponent|SetGravityScale (Variables|Character|GetCharacterMovement) 0.0))

(event EventBeginPlay
  (Variables|Default|SetstartingPoint (Transformation|GetWorldTransform (Variables|Collision|GetCapsuleComponent)))
  (if (Variables|Default|GetTesting)
    _))

(event EventTick
  (params (DeltaSeconds :type Float%20%28single-precision%29))
  ;[1 1 1] Tick Events
  (switch Utilities|FlowControl|Switch|SwitchonEN_EnemyStates (Variables|Default|GetEnumStates)))

(fn ConstructionScript)

(fn GetHurt
  (params (AttackingActor :type Actor%20Object%20Reference))
  (switch Utilities|FlowControl|Switch|SwitchonEN_EnemyStates (Variables|Default|GetEnumStates)
    (:NewEnumerator0
      _)
    (:NewEnumerator8
      _)
    (:NewEnumerator1
      _))
  (Variables|Default|SetEnumStates "NewEnumerator7"))

(fn ResetEnemy
  (bind _startingpoint (Variables|Default|GetstartingPoint))
  (if (Variables|Default|GetTesting)
    _
    (else
      (Utilities|IsValid (Variables|Default|GetSpawnerReference)
        (:Is%20Valid
          _))))
  (Variables|Default|SetEnumStates "NewEnumerator0")
  (Variables|/Script/Engine.MovementComponent|SetVelocity (Variables|Character|GetCharacterMovement) "0, 0, 0")
  (Transformation|SetWorldTransform (Variables|Collision|GetCapsuleComponent) (Math|Transform|MakeTransform (.location _startingpoint) (Math|Rotator|MakeRotator 0.0 0.0 (.yaw (.rotation _startingpoint))) (.scale _startingpoint)) false false)
  (CallFunction|EnableEnemy))

(fn SpawnEnemy
  (CallFunction|ResetEnemy))

(fn CanbeGrabbed
  (return (and (Utilities|Enum|Equal(Enum) (Variables|Default|GetEnumStates) "NewEnumerator7") (<= (Variables|Default|GetinvincibilityCountdown) 0.0))))