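; Mole enemy character that jumps on spotting the player, dash-attacks, and can be thrown into walls to become a platform.
; An EnumStates machine drives reactions: a first hit stuns it, while hits when stunned or stuck rocket it away dying.
; Dash and thrown flight run as per-frame Delay loops.
; When thrown, it flies without gravity, line-tracing for walls to attach to, until a timer restores gravity; landing stuns it.
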(event Custom|ActivateThrownHitbox
  ;[1 1 1] Player Damage Source Activation
  (bind _asbp_damage_source (Utilities|Casting|CastToBP_DamageSource (Variables|/Script/Engine.ChildActorComponent|GetChildActor (Variables|Default|GetThrownHitbox))))
  (Default|ActivateCollision _asbp_damage_source))

(event Custom|DeactivateThrownHitbox
  ;[1 1 1] Player Damage Source Activation
  (bind _asbp_damage_source (Utilities|Casting|CastToBP_DamageSource (Variables|/Script/Engine.ChildActorComponent|GetChildActor (Variables|Default|GetThrownHitbox))))
  (Default|DeactivateCollision _asbp_damage_source))

(event Custom|ActivatePlatform
  ;[1 1 1] Stand In Platform Activation
  (Collision|SetCollisionEnabled (Variables|Default|GetStuckStandOnCollision) "QueryAndPhysics"))

(event Custom|DeactivatePlatform
  ;[1 1 1] Stand In Platform Activation
  (Collision|SetCollisionEnabled (Variables|Default|GetStuckStandOnCollision) "NoCollision"))

(event Custom|ThrownLanding
  ;[1 1 1] Being thrown checks
  (CallFunction|GetHurt))

(event Custom|ThrownFlying
  (bind _returnvalue (Utilities|Time|GetWorldDeltaSeconds))
  ;[1 1 1] Being thrown checks
  (Transformation|DetachFromActor "KeepWorld" "KeepWorld" "KeepWorld")
  (CallFunction|DisableGravity)
  (bind _output_get (Variables|Default|SetLaunchTimeBeforeDescendingCountdown (Variables|Default|GetLaunchTimeBeforeDescending)))
  (if (and (> (Variables|Default|GetLaunchTimeBeforeDescendingCountdown) 0.0) (Utilities|Enum|Equal(Enum) (Variables|Default|GetEnumStates) "NewEnumerator11")) :!label _label
    (Variables|Default|SetLaunchTimeBeforeDescendingCountdown (- _output_get _returnvalue))
    (CallFunction|SticktoWall)
    (Utilities|FlowControl|Delay _returnvalue)
    (goto _label)
    (elif (<= (Variables|Default|GetLaunchTimeBeforeDescendingCountdown) 0.0)
      (CallFunction|EnableGravity))))

(event Custom|SpringBackToAction
  ;[1 1 1] Spring Back to action
  (switch Utilities|FlowControl|Switch|SwitchonEN_EnemyStates (Variables|Default|GetEnumStates)
    (:NewEnumerator7
      (Character|Jump)
      (Utilities|FlowControl|Delay 0.2)
      (Variables|Default|SetEnumStates "NewEnumerator0")
      (CallFunction|ActivateHitbox)
      (CallFunction|EnableGravity))))

(event EventBeginPlay
  (CallFunction|DeactivateHitbox)
  (CallFunction|DeactivateThrownHitbox)
  (CallFunction|DeactivatePlatform)
  (|CallParentFunction))

(event Collision|EventActorBeginOverlap
  (params (OtherActor :type Actor%20Object%20Reference)))

(event EventEnemySpotPlayer
  ;[1 1 1] Blueprint Interfaces
  (Development|PrintString "SPOT")
  (Character|Jump))

(event EventEnemyAttackPlayer
  (bind _returnvalue (Transformation|GetActorForwardVector))
  (bind _returnvalue_2 (Utilities|Time|GetWorldDeltaSeconds))
  (bind _dashspeed (Variables|Default|GetdashSpeed))
  (bind _returnvalue_3 (* _returnvalue _dashspeed))
  ;[1 1 1] Blueprint Interfaces
  (Variables|Default|SetEnumStates "NewEnumerator12")
  (CallFunction|ActivateHitbox)
  (Variables|Default|SetdashCountdown (Variables|Default|GetdashTime))
  (if (> (Variables|Default|GetdashCountdown) 0.0) :!label _label
    (Variables|Default|SetdashCountdown (- (Variables|Default|GetdashCountdown) _returnvalue_2))
    (Utilities|FlowControl|Delay _returnvalue_2)
    (Character|LaunchCharacter _returnvalue_3 true true)
    (goto _label)
    (else
      (Variables|Default|SetEnumStates "NewEnumerator0")
      (Character|LaunchCharacter _returnvalue_3 false true)
      (CallFunction|DeactivateHitbox))))

(event EventOnLanded
  (params (Hit :type Hit%20Result%20Structure%20%28by%20ref%29))
  (switch Utilities|FlowControl|Switch|SwitchonEN_EnemyStates (Variables|Default|GetEnumStates)
    (:NewEnumerator4
      (Variables|Default|SetEnumStates "NewEnumerator5")
      (Utilities|FlowControl|Delay (Variables|Default|GetspawningLagTime))
      (Variables|Default|SetEnumStates "NewEnumerator0"))
    (:NewEnumerator11
      (CallFunction|ThrownLanding))))

(event EventEnableEnemy
  ;[1 1 1] Enable Enemy
  (|CallParentFunction)
  (CallFunction|ActivateHitbox)
  (CallFunction|EnableGravity))

(event EventGetHurt
  (params (AttackingActor :type Actor%20Object%20Reference))
  (bind _returnvalue (Transformation|GetActorLocation AttackingActor))
  (bind _deathrocketinglateralforce (Variables|Default|GetdeathRocketingLateralForce))
  (bind _capsulecomponent (Variables|Default|GetCapsuleComponent))
  (bind _returnvalue_2 (Transformation|GetWorldLocation _capsulecomponent))
  (bind _returnvalue_3 (Math|Vector|GetUnitDirection(Vector) _returnvalue _returnvalue_2))
  (bind _returnvalue_4 (* _returnvalue_3 _deathrocketinglateralforce))
  ;[0 0.7207 1] Mole Getting hit!
  (switch Utilities|FlowControl|Switch|SwitchonEN_EnemyStates (Variables|Default|GetEnumStates)
    (:NewEnumerator0
      (Variables|Default|SetEnumStates "NewEnumerator7" :!label _label)
      ;[1 1 1] Get Flipped
      (Variables|Default|SetstunTimeCountdown (Variables|Default|GetstunTime))
      (Variables|Default|SetinvincibilityCountdown (Variables|Default|GetinvincibilityTime))
      (CallFunction|DeactivateHitbox)
      (CallFunction|InvincibilityTimer)
      (CallFunction|CountStunTimer))
    (:NewEnumerator8
      (goto _label))
    (:NewEnumerator1
      (goto _label))
    (:NewEnumerator7
      (if (not (> 0.0 (Variables|Default|GetinvincibilityTime))) :!label _label_2
        (Variables|Default|SetEnumStates "NewEnumerator2")
        ;[1 1 1] Get killed
        (CallFunction|EnableGravity)
        (CallFunction|DeactivatePlatform)
        (Character|LaunchCharacter (Math|Vector|MakeVector (.x _returnvalue_4) (.y _returnvalue_4) (Variables|Default|GetdeathRocketingVerticalForce)) true true)
        (CallFunction|DisableCollision)))
    (:NewEnumerator11
      (goto _label))
    (:NewEnumerator3
      (goto _label_2))
    (:NewEnumerator13
      (goto _label))))

(event EventTick
  (params (DeltaSeconds :type Float%20%28single-precision%29)))

(fn ConstructionScript
  (|CallParentFunction))

(fn SticktoWall
  (bind _outhit (Collision|LineTraceByChannel (CallFunction|GetWallTraceStartLocation) (CallFunction|GetWallTraceEndLocation) "TraceTypeQuery1" false 0 "ForOneFrame" true "(R=1.000000,G=0.000000,B=0.000000,A=1.000000)" "(R=0.000000,G=1.000000,B=0.000000,A=1.000000)" 0.5))
  (if (.bBlockingHit (Collision|BreakHitResult _outhit))
    (Development|PrintString (Utilities|String|ToString(Vector) (.Normal (Collision|BreakHitResult _outhit))))
    (Transformation|SetWorldRotation (Variables|Default|GetCapsuleComponent) (* (Math|Conversions|RotationFromXVector (.Normal (Collision|BreakHitResult _outhit))) -1.0) false false)
    (Variables|Default|SetEnumStates "NewEnumerator3")
    (CallFunction|DisableGravity)
    (Variables|/Script/Engine.MovementComponent|SetVelocity (Variables|Character|GetCharacterMovement) "0, 0, 0")
    (CallFunction|ActivatePlatform)
    (Transformation|AttachComponentToComponent (.HitComponent (Collision|BreakHitResult _outhit)) "None" "KeepWorld" "KeepWorld" "KeepWorld" true)))

(fn GetWallTraceStartLocation
  (return (Transformation|GetWorldLocation (Variables|Default|GetWallCheck))))

(fn GetWallTraceEndLocation
  (return (+ (CallFunction|GetWallTraceStartLocation) (* (Math|Vector|GetForwardVector (Transformation|GetWorldRotation (Variables|Default|GetWallCheck))) (Variables|Default|GetBumpRange)))))