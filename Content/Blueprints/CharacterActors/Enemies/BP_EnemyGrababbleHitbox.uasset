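; Grabbable hitbox actor for enemies, apparently meant to be a child actor of a BP_EnemyBase.
; On BeginPlay it caches the parent enemy and copies its Damage, printing debug text on success or the parent's name if the cast fails.
; ActivateCollision and DeactivateCollision switch the GrabableBox between query-and-physics and no collision.
; It has no overlap or damage logic of its own.
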(event Custom|Activate%20Collision
  (Collision|SetCollisionEnabled (Variables|Default|GetGrabableBox) "QueryAndPhysics"))

(event Custom|Deactivate%20Collision
  (Collision|SetCollisionEnabled (Variables|Default|GetGrabableBox) "NoCollision"))

(event EventBeginPlay
  (bind _returnvalue (Actor|GetParentActor))
  (bind _asbp_enemy_base (Utilities|Casting|CastToBP_EnemyBase _returnvalue)
    (:then
      (bind _output_get (Variables|Default|SetParentEnemy _asbp_enemy_base))
      (Variables|Default|SetDamage (Variables|/Game/Blueprints/CharacterActors/Enemies/BP_EnemyBase.BP_EnemyBase_C|Getdamage _output_get))
      (Development|PrintString "PArented enemy hitbox"))
    (:CastFailed
      (Development|PrintString (Utilities|GetDisplayName _returnvalue)))))

(event Collision|EventActorBeginOverlap
  (params (OtherActor :type Actor%20Object%20Reference)))

(event EventTick
  (params (DeltaSeconds :type Float%20%28single-precision%29)))

(fn ConstructionScript)