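; BP_EnemyDamageSource is an enemy hitbox actor that damages the player when its DamageHitbox overlaps them.
; On BeginPlay it casts its parent actor to BP_EnemyBase and copies that enemy's Damage value.
; An overlap with a BP_PlayerBase calls the player's GetHit with that damage and itself as the source.
; ActivateCollision and DeactivateCollision events switch the hitbox collision on and off.
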(event OnComponentBeginOverlap(DamageHitbox)
  (params (OverlappedComponent :type Primitive%20Component%20Object%20Reference) (OtherActor :type Actor%20Object%20Reference) (OtherComp :type Primitive%20Component%20Object%20Reference) (OtherBodyIndex :type Integer) (bFromSweep :type Boolean) (SweepResult :type Hit%20Result%20Structure%20%28by%20ref%29))
  ;[1 1 1] Hit Player
  (bind _asbp_player_base (Utilities|Casting|CastToBP_PlayerBase OtherActor))
  (Default|GetHit _asbp_player_base (Variables|Default|GetDamage) self))

(event Custom|Activate%20Collision
  (Collision|SetCollisionEnabled (Variables|Default|GetDamageHitbox) "QueryAndPhysics"))

(event Custom|Deactivate%20Collision
  (Collision|SetCollisionEnabled (Variables|Default|GetDamageHitbox) "NoCollision"))

(event EventBeginPlay
  (bind _returnvalue (Actor|GetParentActor))
  (bind _asbp_enemy_base (Utilities|Casting|CastToBP_EnemyBase _returnvalue)
    (:then
      (bind _output_get (Variables|Default|SetParentEnemy _asbp_enemy_base))
      (Variables|Default|SetDamage (Variables|/Game/Blueprints/CharacterActors/Enemies/BP_EnemyBase.BP_EnemyBase_C|Getdamage _output_get))
      (Development|PrintString "PArented enemy hitbox"))
    (:CastFailed
      (Development|PrintString (Utilities|GetDisplayName _returnvalue)))))

(event Collision|EventActorBeginOverlap
  (params (OtherActor :type Actor%20Object%20Reference)))

(event EventTick
  (params (DeltaSeconds :type Float%20%28single-precision%29)))

(fn ConstructionScript)