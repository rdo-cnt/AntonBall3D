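; Display actor that previews the player's saved character colors on a skeletal mesh.
; On BeginPlay it creates a dynamic material instance on material slot 2 and caches the game instance.
; Every Tick it reads the saved shirt, skin and overalls indices, looks them up in the game instance's color maps, and writes them to material vector parameters, so selection changes show immediately.
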(event Custom|ChangeColor
  (bind _gameinstance (Variables|Default|GetGameInstance))
  (bind _gameinstance_2 (Variables|Default|GetGameInstance))
  (bind _gameinstance_3 (Variables|Default|GetGameInstance))
  ;[0.9711 0 1] Colors
  ;;[0.338 1 0.09807] Shirt
  (bind _values (Utilities|Map|Values (Variables|/Game/Blueprints/BP_AntonGame_GameInstance.BP_AntonGame_GameInstance_C|GetShirtColors _gameinstance)))
  (Rendering|Material|SetVectorParameterValue (Variables|Default|GetBodyMaterialInstance) "ShirtColor" (Math|Conversions|ToLinearColor(Color) (Utilities|Array|Get(acopy) _values (Variables|/Game/Blueprints/SaveGameStuff.SaveGameStuff_C|GetColorShirtIndex (Variables|/Game/Blueprints/BP_AntonGame_GameInstance.BP_AntonGame_GameInstance_C|GetSaveGame _gameinstance)))) :!class /Script/Engine.MaterialInstanceDynamic)
  ;;[1 0 0] Skin
  (bind _values_2 (Utilities|Map|Values (Variables|/Game/Blueprints/BP_AntonGame_GameInstance.BP_AntonGame_GameInstance_C|GetSkinColors _gameinstance_2)))
  (Rendering|Material|SetVectorParameterValue (Variables|Default|GetBodyMaterialInstance) "SkinColor" (Math|Conversions|ToLinearColor(Color) (Utilities|Array|Get(acopy) _values_2 (Variables|/Game/Blueprints/SaveGameStuff.SaveGameStuff_C|GetColorSkinIndex (Variables|/Game/Blueprints/BP_AntonGame_GameInstance.BP_AntonGame_GameInstance_C|GetSaveGame _gameinstance_2)))) :!class /Script/Engine.MaterialInstanceDynamic)
  ;;[0 0 0] Overalls
  (bind _values_3 (Utilities|Map|Values (Variables|/Game/Blueprints/BP_AntonGame_GameInstance.BP_AntonGame_GameInstance_C|GetOverallsColors _gameinstance_3)))
  (Rendering|Material|SetVectorParameterValue (Variables|Default|GetBodyMaterialInstance) "OverallColor" (Math|Conversions|ToLinearColor(Color) (Utilities|Array|Get(acopy) _values_3 (Variables|/Game/Blueprints/SaveGameStuff.SaveGameStuff_C|GetColorOverallsIndex (Variables|/Game/Blueprints/BP_AntonGame_GameInstance.BP_AntonGame_GameInstance_C|GetSaveGame _gameinstance_3)))) :!class /Script/Engine.MaterialInstanceDynamic))

(event Custom|ColorInitialization
  (bind _returnvalue (Rendering|Material|CreateDynamicMaterialInstance (Variables|Default|GetSkeletalMesh) 2 0 "" :!class /Script/Engine.PrimitiveComponent))
  (Variables|Default|SetBodyMaterialInstance _returnvalue))

(event EventBeginPlay
  (CallFunction|ColorInitialization)
  (bind _asbp_anton_game_game_instance (Utilities|Casting|CastToBP_AntonGame_GameInstance (Game|GetGameInstance)))
  (Variables|Default|SetGameInstance _asbp_anton_game_game_instance))

(event Collision|EventActorBeginOverlap
  (params (OtherActor :type Actor%20Object%20Reference)))

(event EventTick
  (params (DeltaSeconds :type Float%20%28single-precision%29))
  (CallFunction|ChangeColor))

(fn ConstructionScript)